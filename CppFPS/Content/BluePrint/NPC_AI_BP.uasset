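; NPC AI controller that starts patrol behavior for its controlled pawn.
; On BeginPlay it sets up the PatrolData blackboard and runs the Patrol behavior tree.
; AI Perception updates only print the pawn, sense class and sensed actor for debugging.
; FindPatrolRoute writes the ThirdPersonCharacter pawn's first PatrolPoint to the Waypoint key, but its call here is disconnected, as are the test vector setters.
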(event `self.ReceiveBeginPlay`
  (`self.UseBlackboard` "/Game/BluePrint/PatrolData.PatrolData")
  (`self.RunBehaviorTree` "/Game/BluePrint/Patrol.Patrol"))

(event `self.AIPerception.OnTargetPerceptionUpdated`
  (params (Actor :type "Actor Object Reference") (Stimulus :type "AIStimulus Structure"))
  (bind _returnvalue (`AIPerceptionSystem.GetSenseClassForStimulus` Stimulus))
  (`KismetSystemLibrary.PrintString` (`KismetStringLibrary.Concat_StrStr` (`KismetSystemLibrary.GetObjectName` (`self.K2_GetPawn`)) " " (`KismetSystemLibrary.GetClassDisplayName` _returnvalue) " " (`KismetSystemLibrary.GetObjectName` Actor))))

(fn `FindPatrolRoute`
  (params (self2 :type "BlackboardComponent Object Reference"))
  (`BlackboardComponent.SetValueAsObject` self2 "Waypoint" (`KismetArrayLibrary.Array_Get` (`/Game/ThirdPersonCPP/Blueprints/ThirdPersonCharacter.PatrolPoint` (cast `/Game/ThirdPersonCPP/Blueprints/ThirdPersonCharacter` (`self.K2_GetPawn`) :!pure true)))))

(fn `UserConstructionScript`)